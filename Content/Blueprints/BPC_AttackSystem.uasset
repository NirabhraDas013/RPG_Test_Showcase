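; Attack component for the third-person character that runs a four-step melee combo of sword attacks and a kick.
; Input starts a montage or buffers the next attack, which SwordAttackCombo plays or otherwise resets the combo.
; A looping timer sphere-traces along the blade, while GeneralAttackTrace makes single checks for stab and kick.
; Both damage actors tagged Damagable, with sword hits throttled and adding camera shake, sound and blood.
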(event Custom|SwordAttack
  ;[0.05098 0.05098 0.05098] ComboSystem
  ;;[0.05098 0.05098 0.05098] SwordAttack
  (if (Variables|Default|GetisAttacking?)
    (Variables|Default|SetsaveAttack? true)
    (else
      (Variables|Default|SetisAttacking? true)
      (switch int (Variables|Default|GetAttackIndex)
        (:0
          (CallFunction|Attack00))
        (:1
          (CallFunction|Attack01))
        (:2
          (CallFunction|Attack02))
        (:3
          (CallFunction|Attack03))))))

(event Custom|SwordAttackCombo
  ;[0.05098 0.05098 0.05098] ComboSystem
  ;;[0.05098 0.05098 0.05098] SwordAttackCombo
  (if (Variables|Default|GetsaveAttack?)
    (Variables|Default|SetsaveAttack? false)
    (switch int (Variables|Default|GetAttackIndex)
      (:0
        (CallFunction|Attack00))
      (:1
        (CallFunction|Attack01))
      (:2
        (CallFunction|Attack02))
      (:3
        (CallFunction|Attack03)))
    (else
      (CallFunction|StopCombo))))

(event Custom|StartSwordTrace
  ;[0.05098 0.05098 0.05098] SwordTrace
  (bind _returnvalue (Utilities|Time|SetTimerbyEvent (delegate Custom|SwordTraceLoop) 0.001 true))
  (Variables|Default|SetSwordTraceTimer _returnvalue))

(event Custom|SwordTraceLoop
  (bind _characterbp (Variables|Default|GetCharacterBP))
  ;[0.05098 0.05098 0.05098] SwordTrace
  (bind (_outhit _returnvalue) (Collision|SphereTraceByChannel (Transformation|GetWorldLocation (Variables|/Game/ThirdPerson/Blueprints/BP_ThirdPersonCharacter.BP_ThirdPersonCharacter_C|GetSwordTopPoint _characterbp)) (Transformation|GetWorldLocation (Variables|/Game/ThirdPerson/Blueprints/BP_ThirdPersonCharacter.BP_ThirdPersonCharacter_C|GetSwordBasePoint _characterbp)) 12.0 "TraceTypeQuery1" false 0 "None" true "(R=1.000000,G=0.000000,B=0.000000,A=1.000000)" "(R=0.000000,G=1.000000,B=0.000000,A=1.000000)" 0.1))
  (CallFunction|DamageEnemy _outhit _returnvalue true))

(event Custom|StopSwordTrace
  ;[0.05098 0.05098 0.05098] SwordTrace
  (Utilities|Time|ClearandInvalidateTimerbyHandle (Variables|Default|GetSwordTraceTimer)))

(event Custom|GeneralAttackTrace
  (bind _characterbp (Variables|Default|GetCharacterBP))
  (bind _generalattacktrace (Variables|/Game/ThirdPerson/Blueprints/BP_ThirdPersonCharacter.BP_ThirdPersonCharacter_C|GetGeneralAttackTrace _characterbp))
  (bind _returnvalue (Transformation|GetWorldLocation _generalattacktrace))
  ;[0.05098 0.05098 0.05098] GeneralAttacktrace(For Stab and Kick)
  (bind (_outhit _returnvalue_2) (Collision|SphereTraceByChannel _returnvalue _returnvalue 25.0 "TraceTypeQuery1" false 0 "None" true "(R=1.000000,G=0.000000,B=0.000000,A=1.000000)" "(R=0.000000,G=1.000000,B=0.000000,A=1.000000)" 0.3))
  (CallFunction|DamageEnemy _outhit _returnvalue_2 false))

(event Custom|DamageEnemy
  (params (Hit :type Hit%20Result%20Structure%20%28by%20ref%29) (HitReturn? :type Boolean) (IsInLoop? :type Boolean))
  (bind (_bblockinghit _binitialoverlap _time _distance _location _impactpoint _normal _impactnormal _physmat _hitactor) (Collision|BreakHitResult Hit))
  ;[0.05098 0.05098 0.05098] DamageEnemyFromHitTrace
  (if HitReturn?
    (if (Actor|ActorHasTag _hitactor "Damagable")
      (if IsInLoop?
        (Utilities|FlowControl|DoOnce false :!label _label
          (:Completed
            _)))
      (Game|Damage|ApplyDamage _hitactor 1e+01 0 0)
      (if IsInLoop?
        (Camera|PlayWorldCameraShake "/Game/Blueprints/BP_SwordHitCameraShake.BP_SwordHitCameraShake_C" _location 0.0 2e+03)
        (CallFunction|PlaySwordHitSound)
        (Effects|SpawnEmitteratLocation "/Game/VFX/Particles/Blood/P_Blood_Splat_Cone.P_Blood_Splat_Cone" _location (Math|Rotator|MakeRotfromXY _normal _normal) "0.400000,0.400000,0.400000" true "AutoRelease")
        (Utilities|FlowControl|Delay 0.5)
        (goto _label Reset)))))

(event Custom|PlaySwordHitSound
  ;[0.05098 0.05098 0.05098] PlaySwordHitSounds
  (Audio|PlaySoundatLocation "/Game/Audio/SwordHits/MS_SwordHit.MS_SwordHit" (Transformation|GetActorLocation (Components|GetOwner)) "0, 0, 0" 1.0 1.0 0.0 "/Game/Audio/SA_CharacterOverall.SA_CharacterOverall" 0 0 0))

(event Custom|StopCombo
  ;[0.05098 0.05098 0.05098] ComboSystem
  ;;[0.05098 0.05098 0.05098] Stop Combo Attack
  (Variables|Default|SetisAttacking? false)
  (Variables|Default|SetAttackIndex 0))

(event Custom|Attack03
  ;[0.05098 0.05098 0.05098] ComboSystem
  ;;[0.05098 0.05098 0.05098] Attack03
  (Utilities|FlowControl|DoOnce false :!label _label
    (:Completed
      (Utilities|FlowControl|Delay 0.1)
      (Animation|Montage|PlayMontage (Variables|Default|GetCharacterMesh) "/Game/Characters/RPG_Character/Animations/SwordAttacks/Attack3_Montage.Attack3_Montage"
        (:then
          (Variables|Default|SetAttackIndex 4)
          (goto _label Reset))))))

(event Custom|Attack00
  ;[0.05098 0.05098 0.05098] ComboSystem
  ;;[0.05098 0.05098 0.05098] Attack00
  (Utilities|FlowControl|DoOnce false :!label _label
    (:Completed
      (Utilities|FlowControl|Delay 0.1)
      (Animation|Montage|PlayMontage (Variables|Default|GetCharacterMesh) "/Game/Characters/RPG_Character/Animations/SwordAttacks/Attack1_Montage.Attack1_Montage"
        (:then
          (Variables|Default|SetAttackIndex 1)
          (goto _label Reset))))))

(event Custom|Attack01
  ;[0.05098 0.05098 0.05098] ComboSystem
  ;;[0.05098 0.05098 0.05098] Attack01
  (Utilities|FlowControl|DoOnce false :!label _label
    (:Completed
      (Utilities|FlowControl|Delay 0.1)
      (Animation|Montage|PlayMontage (Variables|Default|GetCharacterMesh) "/Game/Characters/RPG_Character/Animations/SwordAttacks/Attack2_Montage.Attack2_Montage"
        (:then
          (Variables|Default|SetAttackIndex 2)
          (goto _label Reset))))))

(event Custom|Attack02
  ;[0.05098 0.05098 0.05098] ComboSystem
  ;;[0.05098 0.05098 0.05098] Attack03
  (Utilities|FlowControl|DoOnce false :!label _label
    (:Completed
      (Utilities|FlowControl|Delay 0.1)
      (Animation|Montage|PlayMontage (Variables|Default|GetCharacterMesh) "/Game/Characters/RPG_Character/Animations/SwordAttacks/Kick_Montage.Kick_Montage"
        (:then
          (Variables|Default|SetAttackIndex 3)
          (goto _label Reset))))))

(event Input|EnhancedActionEvents|EnhancedInputActionIA_Attack
  (params (ActionValue :type Boolean) (ElapsedSeconds :type Float%20%28double-precision%29) (TriggeredSeconds :type Float%20%28double-precision%29) (InputAction :type Input%20Action%20Object%20Reference :default "/Game/ThirdPerson/Input/Actions/IA_Attack.IA_Attack"))
  ;[0.05098 0.05098 0.05098] ComboSystem
  ;;[0.05098 0.05098 0.05098] AttackInput
  (:Started
    (if (Variables|Default|GetcanAttack?)
      (CallFunction|SwordAttack))))

(event EventBeginPlay
  (bind _asbp_third_person_character (Utilities|Casting|CastToBP_ThirdPersonCharacter (Components|GetOwner)))
  (Variables|Default|SetCharacterBP _asbp_third_person_character)
  (Variables|Default|SetCharacterMesh (Variables|/Script/Engine.Character|GetMesh _asbp_third_person_character)))