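; Stats component for the player, dummy and AI characters, tracking health, plus stamina, XP and level for the player.
; On BeginPlay it waits a tick, casts its owner and fills that owner's widgets.
; Stat functions update values and push bars and text directly, but health changes always target the dummy's widget.
; Enough XP triggers a level-up that resets XP, raises its cap and plays sounds.
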(event Custom|SetHealthText
  (params (IsPlayer? :type Boolean) (IsAI? :type Boolean))
  ;[0.05098 0.05098 0.05098] SetTextAndPercents
  (bind _healthamounttext (Health|GetHealthText IsPlayer? IsAI?))
  (Rendering|Components|TextRender|SetText _healthamounttext (Utilities|Text|FormatText "{CurrentHealth}/{MaxHealth}" (Variables|Health|GetCurrentHealth) (Variables|Health|GetMaxHealth))))

(event Custom|SetStaminaText
  ;[0.05098 0.05098 0.05098] SetTextAndPercents
  (bind _healthamounttext (Stamina|GetStaminaText))
  (Rendering|Components|TextRender|SetText _healthamounttext (Utilities|Text|FormatText "{CurrentStamina}/{MaxStamina}" (Variables|Stamina|GetCurrentStamina) (Variables|Stamina|GetMaxStamina))))

(event Custom|SetHealthPercent
  (params (IsPlayer? :type Boolean) (IsAI? :type Boolean))
  ;[0.05098 0.05098 0.05098] SetTextAndPercents
  (bind _healthpercent (Health|GetHealthPercent))
  (bind _healthbar (Health|GetHealthBar IsPlayer? IsAI?))
  (Progress|SetPercent _healthbar _healthpercent))

(event Custom|SetStaminaPercent
  ;[0.05098 0.05098 0.05098] SetTextAndPercents
  (bind _staminapercent (Stamina|GetStaminaPercent))
  (bind _staminabar (Stamina|GetStaminaBar))
  (Progress|SetPercent _staminabar _staminapercent))

(event Custom|SetXPPercent
  ;[0.05098 0.05098 0.05098] SetTextAndPercents
  (bind _xppercent (Experience|GetXpPercent))
  (bind _xpbar (Experience|GetXpBar))
  (Progress|SetPercent _xpbar _xppercent))

(event Custom|SetXPText
  ;[0.05098 0.05098 0.05098] SetTextAndPercents
  (bind _xptext (Experience|GetXPText))
  (Rendering|Components|TextRender|SetText _xptext (Utilities|Text|FormatText "{CurrentXP}/{MaxXP}" (Variables|Experience|GetXP) (Variables|Experience|GetMaxXP))))

(event Custom|SetLevelText
  ;[0.05098 0.05098 0.05098] SetTextAndPercents
  (bind _leveltext (Experience|GetLevelText))
  (Rendering|Components|TextRender|SetText _leveltext (Utilities|Text|ToText(Integer) (Variables|Experience|GetLevel))))

(event EventBeginPlay
  (Utilities|FlowControl|DelayUntilNextTick)
  (bind _asbp_third_person_character (Utilities|Casting|CastToBP_ThirdPersonCharacter (Components|GetOwner))
    (:then
      (Variables|Default|SetPlayerCharacterBP _asbp_third_person_character)
      (CallFunction|SetHealthPercent true false)
      (CallFunction|SetHealthText true false)
      (CallFunction|SetStaminaPercent)
      (CallFunction|SetStaminaText)
      (CallFunction|SetXPPercent)
      (CallFunction|SetXPText)
      (CallFunction|SetLevelText))
    (:CastFailed
      (bind _asbp_dummy (Utilities|Casting|CastToBP_Dummy (Components|GetOwner))
        (:then
          (Variables|Default|SetDummyBP _asbp_dummy)
          (CallFunction|SetHealthPercent false false)
          (CallFunction|SetHealthText false false))
        (:CastFailed
          (bind _asbp_ai (Utilities|Casting|CastToBP_AI (Components|GetOwner)))
          (Variables|Default|SetAIBP _asbp_ai)
          (CallFunction|SetHealthPercent false true)
          (CallFunction|SetHealthText false true))))))

(event EventTick
  (params (DeltaSeconds :type Float%20%28single-precision%29)))

(fn DecreaseHealth
  (params (Amount :type Float%20%28double-precision%29))
  (if (> (Variables|Health|GetCurrentHealth) 0.0)
    (bind _output_get (Variables|Health|SetCurrentHealth (- (Variables|Health|GetCurrentHealth) Amount)))
    (bind _healthpercent (Health|GetHealthPercent))
    (bind _healthbar (Health|GetHealthBar false false))
    (Progress|SetPercent _healthbar _healthpercent)
    (bind _healthamounttext (Health|GetHealthText false false))
    (Rendering|Components|TextRender|SetText _healthamounttext (Utilities|Text|FormatText "{CurrentHealth}/{MaxHealth}" _output_get (Variables|Health|GetMaxHealth)))
    (if (<= _output_get 0.0)
      (return true)
      (else
        (return false)))))

(fn IncreaseMaxHealth
  (params (Amount :type Float%20%28double-precision%29))
  (bind _output_get (Variables|Health|SetMaxHealth (+ Amount (Variables|Health|GetMaxHealth))))
  (bind _healthpercent (Health|GetHealthPercent))
  (bind _healthbar (Health|GetHealthBar false false))
  (Progress|SetPercent _healthbar _healthpercent)
  (bind _healthamounttext (Health|GetHealthText false false))
  (Rendering|Components|TextRender|SetText _healthamounttext (Utilities|Text|FormatText "{CurrentHealth}/{MaxHealth}" (Variables|Health|GetCurrentHealth) _output_get)))

(fn DecreaseStamina
  (params (Amount :type Float%20%28double-precision%29))
  (if (> (Variables|Stamina|GetCurrentStamina) 0.0)
    (bind _output_get (Variables|Stamina|SetCurrentStamina (- (Variables|Stamina|GetCurrentStamina) Amount)))
    (bind _staminapercent (Stamina|GetStaminaPercent))
    (bind _staminabar (Stamina|GetStaminaBar))
    (Progress|SetPercent _staminabar _staminapercent)
    (bind _healthamounttext (Stamina|GetStaminaText))
    (Rendering|Components|TextRender|SetText _healthamounttext (Utilities|Text|FormatText "{CurrentStamina}/{MaxStamina}" _output_get (Variables|Stamina|GetMaxStamina)))
    (if (<= _output_get 0.0)
      (return true)
      (else
        (return false)))))

(fn IncreaseMaxStamina
  (params (Amount :type Float%20%28double-precision%29))
  (bind _output_get (Variables|Stamina|SetMaxStamina (+ Amount (Variables|Stamina|GetMaxStamina))))
  (bind _staminapercent (Stamina|GetStaminaPercent))
  (bind _staminabar (Stamina|GetStaminaBar))
  (Progress|SetPercent _staminabar _staminapercent)
  (bind _healthamounttext (Stamina|GetStaminaText))
  (Rendering|Components|TextRender|SetText _healthamounttext (Utilities|Text|FormatText "{CurrentStamina}/{MaxStamina}" (Variables|Stamina|GetCurrentStamina) _output_get)))

(fn IncreaseHealth
  (params (Amount :type Float%20%28double-precision%29))
  (bind _output_get (Variables|Health|SetCurrentHealth (Math|Float|Clamp(Float) (+ Amount (Variables|Health|GetCurrentHealth)) 0.0 (Variables|Health|GetMaxHealth))))
  (bind _healthpercent (Health|GetHealthPercent))
  (bind _healthbar (Health|GetHealthBar false false))
  (Progress|SetPercent _healthbar _healthpercent)
  (bind _healthamounttext (Health|GetHealthText false false))
  (Rendering|Components|TextRender|SetText _healthamounttext (Utilities|Text|FormatText "{CurrentHealth}/{MaxHealth}" _output_get (Variables|Health|GetMaxHealth))))

(fn IncreaseStamina
  (params (Amount :type Float%20%28double-precision%29))
  (bind _maxstamina (Variables|Stamina|GetMaxStamina))
  (bind _output_get (Variables|Stamina|SetCurrentStamina (Math|Float|Clamp(Float) (+ Amount (Variables|Stamina|GetCurrentStamina)) 0.0 (Variables|Stamina|GetMaxStamina))))
  (bind _staminapercent (Stamina|GetStaminaPercent))
  (bind _staminabar (Stamina|GetStaminaBar))
  (Progress|SetPercent _staminabar _staminapercent)
  (bind _healthamounttext (Stamina|GetStaminaText))
  (Rendering|Components|TextRender|SetText _healthamounttext (Utilities|Text|FormatText "{CurrentStamina}/{MaxStamina}" _output_get _maxstamina))
  (if (<= _maxstamina _output_get)
    (return true)
    (else
      (return false))))

(fn GetHealthBar
  (params (IsPlayer? :type Boolean) (IsAI? :type Boolean))
  (if IsPlayer?
    (return (Variables|/Game/UI/WB_HUD.WB_HUD_C|GetHealthBar (Variables|/Game/ThirdPerson/Blueprints/BP_ThirdPersonCharacter.BP_ThirdPersonCharacter_C|GetHUDWidget (Variables|Default|GetPlayerCharacterBP))))
    (elif IsAI?
      (return (Variables|/Game/UI/WB_NPC_HealthBar.WB_NPC_HealthBar_C|GetHealthBar (Variables|/Game/AI/BP_AI.BP_AI_C|GetHealthBar (Variables|Default|GetAIBP))))
      (else
        (return (Variables|/Game/UI/WB_NPC_HealthBar.WB_NPC_HealthBar_C|GetHealthBar (Variables|/Game/Blueprints/BP_Dummy.BP_Dummy_C|GetDummyHealthBar (Variables|Default|GetDummyBP))))))))

(fn GetStaminaBar
  (return (Variables|/Game/UI/WB_HUD.WB_HUD_C|GetStaminaBar (Variables|/Game/ThirdPerson/Blueprints/BP_ThirdPersonCharacter.BP_ThirdPersonCharacter_C|GetHUDWidget (Variables|Default|GetPlayerCharacterBP)))))

(fn GetHealthPercent
  (return (/ (Variables|Health|GetCurrentHealth) (Variables|Health|GetMaxHealth))))

(fn GetStaminaPercent
  (return (/ (Variables|Stamina|GetCurrentStamina) (Variables|Stamina|GetMaxStamina))))

(fn GetHealthText
  (params (IsPlayer? :type Boolean) (IsAI :type Boolean))
  (if IsPlayer?
    (return (Variables|/Game/UI/WB_HUD.WB_HUD_C|GetHealthAmountText (Variables|/Game/ThirdPerson/Blueprints/BP_ThirdPersonCharacter.BP_ThirdPersonCharacter_C|GetHUDWidget (Variables|Default|GetPlayerCharacterBP))))
    (elif IsAI
      (return (Variables|/Game/UI/WB_NPC_HealthBar.WB_NPC_HealthBar_C|GetHealthText (Variables|/Game/AI/BP_AI.BP_AI_C|GetHealthBar (Variables|Default|GetAIBP))))
      (else
        (return (Variables|/Game/UI/WB_NPC_HealthBar.WB_NPC_HealthBar_C|GetHealthText (Variables|/Game/Blueprints/BP_Dummy.BP_Dummy_C|GetDummyHealthBar (Variables|Default|GetDummyBP))))))))

(fn GetStaminaText
  (return (Variables|/Game/UI/WB_HUD.WB_HUD_C|GetStaminaAmountText (Variables|/Game/ThirdPerson/Blueprints/BP_ThirdPersonCharacter.BP_ThirdPersonCharacter_C|GetHUDWidget (Variables|Default|GetPlayerCharacterBP)))))

(fn IncreaseXP
  (params (Amount :type Float%20%28double-precision%29))
  (bind _maxxp (Variables|Experience|GetMaxXP))
  (bind _output_get (Variables|Experience|SetXP (+ Amount (Variables|Experience|GetXP))))
  (if (>= _output_get _maxxp)
    (Experience|IncreaseLevel 1))
  (bind _xppercent (Experience|GetXpPercent))
  (bind _xpbar (Experience|GetXpBar))
  (Progress|SetPercent _xpbar _xppercent)
  (bind _xptext (Experience|GetXPText))
  (Rendering|Components|TextRender|SetText _xptext (Utilities|Text|FormatText "{CurrentXP}/{MaxXP}" _output_get _maxxp)))

(fn IncreaseLevel
  (params (AddedLevel :type Integer))
  (bind _output_get (Variables|Experience|SetLevel (+ AddedLevel (Variables|Experience|GetLevel))))
  (bind _leveltext (Experience|GetLevelText))
  (Rendering|Components|TextRender|SetText _leveltext (Utilities|Text|ToText(Integer) _output_get))
  (Variables|Experience|SetMaxXP (+ (Variables|Experience|GetMaxXP) 1.5e+02))
  (Variables|Experience|SetXP 0.0)
  (bind _xppercent (Experience|GetXpPercent))
  (bind _xpbar (Experience|GetXpBar))
  (Progress|SetPercent _xpbar _xppercent)
  (bind _xptext (Experience|GetXPText))
  (Rendering|Components|TextRender|SetText _xptext (Utilities|Text|FormatText "{CurrentXP}/{MaxXP}" (Variables|Experience|GetXP) (Variables|Experience|GetMaxXP)))
  (Audio|PlaySound2D "/Game/Audio/UI/LevelUp01.LevelUp01" 1.0 1.0 0.0 0 0)
  (Audio|PlaySound2D "/Game/Audio/UI/levelUp02.levelUp02" 1.0 1.0 0.0 0 0))

(fn GetXpBar
  (return (Variables|/Game/UI/WB_HUD.WB_HUD_C|GetXPBar (Variables|/Game/ThirdPerson/Blueprints/BP_ThirdPersonCharacter.BP_ThirdPersonCharacter_C|GetHUDWidget (Variables|Default|GetPlayerCharacterBP)))))

(fn GetXPText
  (return (Variables|/Game/UI/WB_HUD.WB_HUD_C|GetXPText (Variables|/Game/ThirdPerson/Blueprints/BP_ThirdPersonCharacter.BP_ThirdPersonCharacter_C|GetHUDWidget (Variables|Default|GetPlayerCharacterBP)))))

(fn GetLevelText
  (return (Variables|/Game/UI/WB_HUD.WB_HUD_C|GetLevelText (Variables|/Game/ThirdPerson/Blueprints/BP_ThirdPersonCharacter.BP_ThirdPersonCharacter_C|GetHUDWidget (Variables|Default|GetPlayerCharacterBP)))))

(fn GetXpPercent
  (return (/ (Variables|Experience|GetXP) (Variables|Experience|GetMaxXP))))