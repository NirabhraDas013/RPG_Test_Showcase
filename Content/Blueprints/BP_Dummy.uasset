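; BP_Dummy is a target dummy character that can be damaged or stealth-assassinated from behind by the player.
; Damage plays a random hit montage, launches it along the player's facing and reduces health via BPCPlayerStats, ragdolling on death.
; An overlap radius toggles an assassination prompt; StealthBackAssassination plays a paired victim montage, returns the attacker's placement and triggers delayed ragdoll.
; A world-space health bar turns toward the camera each tick.
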(event OnComponentBeginOverlap(AssassinationRadius)
  (params (OverlappedComponent :type Primitive%20Component%20Object%20Reference) (OtherActor :type Actor%20Object%20Reference) (OtherComp :type Primitive%20Component%20Object%20Reference) (OtherBodyIndex :type Integer) (bFromSweep :type Boolean) (SweepResult :type Hit%20Result%20Structure%20%28by%20ref%29))
  ;[0.05098 0.05098 0.05098] ToggleAssassinationPrompt
  (Utilities|Casting|CastToBP_ThirdPersonCharacter OtherActor)
  (Rendering|SetVisibility (Variables|Default|GetAssassinatePromptWidget) true false))

(event OnComponentEndOverlap(AssassinationRadius)
  (params (OverlappedComponent :type Primitive%20Component%20Object%20Reference) (OtherActor :type Actor%20Object%20Reference) (OtherComp :type Primitive%20Component%20Object%20Reference) (OtherBodyIndex :type Integer))
  ;[0.05098 0.05098 0.05098] ToggleAssassinationPrompt
  (Utilities|Casting|CastToBP_ThirdPersonCharacter OtherActor)
  (Rendering|SetVisibility (Variables|Default|GetAssassinatePromptWidget) false false))

(event Custom|Ragdoll
  (params (RagdollWaitDuration :type Float%20%28single-precision%29) (DeathSoundWaitDuration :type Float%20%28single-precision%29))
  (bind _mesh (Variables|Character|GetMesh))
  (bind _capsulecomponent (Variables|Collision|GetCapsuleComponent))
  ;[0.05098 0.05098 0.05098] Ragdoll
  (Utilities|FlowControl|Sequence
    (:then_0
      (Utilities|FlowControl|Delay RagdollWaitDuration)
      (Physics|SetSimulatePhysics _mesh true)
      (Collision|SetCollisionObjectType _mesh "ECC_Pawn")
      (Collision|SetCollisionResponsetoChannel _mesh "ECC_Pawn" "ECR_Ignore")
      (Collision|SetCollisionEnabled (Variables|Default|GetAssassinationRadius) "NoCollision")
      (Collision|SetCollisionObjectType _capsulecomponent "ECC_Pawn")
      (Collision|SetCollisionResponsetoChannel _capsulecomponent "ECC_Camera" "ECR_Ignore")
      (Collision|SetCollisionResponsetoChannel _capsulecomponent "ECC_Pawn" "ECR_Ignore"))
    (:then_1
      (Utilities|FlowControl|Delay DeathSoundWaitDuration)
      (Audio|PlaySoundatLocation "/Game/Audio/HitGrunts/Death02.Death02" (Transformation|GetActorLocation) "0, 0, 0" 1.0 1.0 0.0 "/Game/Audio/SA_CharacterOverall.SA_CharacterOverall" 0 0 0)
      (Development|SetHiddeninGame (Variables|Default|GetHealthBarWidget) true true))))

(event EventBeginPlay
  (bind _aswb_dummy_health_bar (Utilities|Casting|CastToWB_DummyHealthBar (UserInterface|GetWidget (Variables|Default|GetHealthBarWidget))))
  (Variables|Default|SetDummyHealthBar _aswb_dummy_health_bar))

(event EventTick
  (params (DeltaSeconds :type Float%20%28single-precision%29))
  (Transformation|SetWorldRotation (Variables|Default|GetHealthBarWidget) (Math|Rotator|FindLookatRotation (Transformation|GetWorldLocation (Variables|Default|GetHealthBarWidget)) (Transformation|GetWorldLocation (Variables|/Script/Engine.PlayerCameraManager|GetTransformComponent (Game|GetPlayerCameraManager 0)))) false false))

(event Game|Damage|EventAnyDamage
  (params (Damage :type Float%20%28single-precision%29) (DamageType :type Damage%20Type%20Object%20Reference) (InstigatedBy :type Controller%20Object%20Reference) (DamageCauser :type Actor%20Object%20Reference))
  (bind _hitanims (Variables|Default|GetHitAnims))
  (Animation|PlayAnimMontage (Utilities|Array|Get(acopy) _hitanims (Math|Random|RandomIntegerinRange 0 (- (Utilities|Array|Length _hitanims) 1))) 1.0 "None")
  (bind _asbp_third_person_character (Utilities|Casting|CastToBP_ThirdPersonCharacter (Game|GetPlayerCharacter 0)))
  (Character|LaunchCharacter (* (Math|Vector|GetForwardVector (Transformation|GetActorRotation _asbp_third_person_character)) 7e+02) false false)
  (Audio|PlaySoundatLocation "/Game/Audio/HitGrunts/Death01.Death01" (Transformation|GetActorLocation) "0, 0, 0" 1.0 1.0 0.0 "/Game/Audio/SA_CharacterOverall.SA_CharacterOverall" 0 0 0)
  (bind _isdead (Default|DecreaseHealth (Variables|Default|GetBPC_PlayerStats) Damage))
  (if _isdead
    (CallFunction|Ragdoll 0.0 0.0)))

(fn ConstructionScript)

(fn StealthBackAssassination
  (Rendering|SetVisibility (Variables|Default|GetAssassinatePromptWidget) false false)
  (Animation|PlayAnimMontage "/Game/Characters/RPG_Character/Animations/Assassinations/Paired_Knife_Stealth_KidneyAndNeck_Vic_Montage.Paired_Knife_Stealth_KidneyAndNeck_Vic_Montage" 1.0 "None")
  (CallFunction|Ragdoll 2.5 2.0)
  (return (Transformation|GetWorldLocation (Variables|Default|GetAssassinREF)) (Transformation|GetActorRotation)))