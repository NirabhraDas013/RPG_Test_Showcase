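; Enemy AI character that fights with a sword, shows health and investigation widgets, and can be stealth-assassinated from behind.
; Attacks chain montages by index with buffered input, while a looping timer sphere-traces the blade to damage tagged actors.
; Incoming damage plays hit reactions, launches the character and reduces health through a stats component, ragdolling on death.
; An overlap radius toggles the assassination prompt, and assassination plays a victim montage before a delayed ragdoll.
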(event OnComponentBeginOverlap(AssassinationRadius)
  (params (OverlappedComponent :type Primitive%20Component%20Object%20Reference) (OtherActor :type Actor%20Object%20Reference) (OtherComp :type Primitive%20Component%20Object%20Reference) (OtherBodyIndex :type Integer) (bFromSweep :type Boolean) (SweepResult :type Hit%20Result%20Structure%20%28by%20ref%29))
  ;[0.05098 0.05098 0.05098] ToggleAssassinationPrompt
  (Utilities|Casting|CastToBP_ThirdPersonCharacter OtherActor)
  (Rendering|SetVisibility (Variables|Default|GetAssassinatePromptWidget) true false))

(event OnComponentEndOverlap(AssassinationRadius)
  (params (OverlappedComponent :type Primitive%20Component%20Object%20Reference) (OtherActor :type Actor%20Object%20Reference) (OtherComp :type Primitive%20Component%20Object%20Reference) (OtherBodyIndex :type Integer))
  ;[0.05098 0.05098 0.05098] ToggleAssassinationPrompt
  (Utilities|Casting|CastToBP_ThirdPersonCharacter OtherActor)
  (Rendering|SetVisibility (Variables|Default|GetAssassinatePromptWidget) false false))

(event Custom|SwordAttack
  ;[0.05098 0.05098 0.05098] ComboSystem
  ;;[0.05098 0.05098 0.05098] SwordAttack
  (if (Variables|Default|GetisAttacking?)
    (Variables|Default|SetsaveAttack? true)
    (else
      (Variables|Default|SetisAttacking? true)
      (switch int (Variables|Default|GetAttackIndex)
        (:0
          (CallFunction|Attack00))
        (:1
          (CallFunction|Attack01))
        (:2
          (CallFunction|Attack03))))))

(event Custom|SwordAttackCombo
  ;[0.05098 0.05098 0.05098] ComboSystem
  ;;[0.05098 0.05098 0.05098] SwordAttackCombo
  (if (Variables|Default|GetsaveAttack?)
    (Variables|Default|SetsaveAttack? false)
    (switch int (Variables|Default|GetAttackIndex)
      (:0
        (CallFunction|Attack00))
      (:1
        (CallFunction|Attack01))
      (:2
        (CallFunction|Attack03)))
    (else
      (CallFunction|StopCombo))))

(event Custom|StartSwordTrace
  ;[0.05098 0.05098 0.05098] SwordTrace
  (bind _returnvalue (Utilities|Time|SetTimerbyEvent (delegate Custom|SwordTraceLoop) 0.001 true))
  (Variables|Default|SetSwordTraceTimer _returnvalue))

(event Custom|SwordTraceLoop
  ;[0.05098 0.05098 0.05098] SwordTrace
  (bind (_outhit _returnvalue) (Collision|SphereTraceByChannel (Transformation|GetWorldLocation (Variables|Default|GetSwordTopPoint)) (Transformation|GetWorldLocation (Variables|Default|GetSwordBasePoint)) 12.0 "TraceTypeQuery1" false 0 "None" true "(R=1.000000,G=0.000000,B=0.000000,A=1.000000)" "(R=0.000000,G=1.000000,B=0.000000,A=1.000000)" 0.1))
  (CallFunction|DamageEnemy _outhit _returnvalue true))

(event Custom|StopSwordTrace
  ;[0.05098 0.05098 0.05098] SwordTrace
  (Utilities|Time|ClearandInvalidateTimerbyHandle (Variables|Default|GetSwordTraceTimer)))

(event Custom|GeneralAttackTrace
  (bind _stabattacktrace (Variables|Default|GetStabAttackTrace))
  (bind _returnvalue (Transformation|GetWorldLocation _stabattacktrace))
  ;[0.05098 0.05098 0.05098] GeneralAttacktrace(For Stab and Kick)
  (bind (_outhit _returnvalue_2) (Collision|SphereTraceByChannel _returnvalue _returnvalue 25.0 "TraceTypeQuery1" false 0 "None" true "(R=1.000000,G=0.000000,B=0.000000,A=1.000000)" "(R=0.000000,G=1.000000,B=0.000000,A=1.000000)" 0.3))
  (CallFunction|DamageEnemy _outhit _returnvalue_2 false))

(event Custom|DamageEnemy
  (params (Hit :type Hit%20Result%20Structure%20%28by%20ref%29) (HitReturn? :type Boolean) (IsInLoop? :type Boolean))
  (bind (_bblockinghit _binitialoverlap _time _distance _location _impactpoint _normal _impactnormal _physmat _hitactor) (Collision|BreakHitResult Hit))
  ;[0.05098 0.05098 0.05098] DamageEnemyFromHitTrace
  (if HitReturn?
    (if (Actor|ActorHasTag _hitactor "Damagable")
      (if IsInLoop?
        (Utilities|FlowControl|DoOnce false :!label _label
          (:Completed
            _)))
      (Game|Damage|ApplyDamage _hitactor 1e+01 0 0)
      (if IsInLoop?
        (Camera|PlayWorldCameraShake "/Game/Blueprints/BP_SwordHitCameraShake.BP_SwordHitCameraShake_C" _location 0.0 2e+03)
        (CallFunction|PlaySwordHitSound)
        (Effects|SpawnEmitteratLocation "/Game/VFX/Particles/Blood/P_Blood_Splat_Cone.P_Blood_Splat_Cone" _location (Math|Rotator|MakeRotfromXY _normal _normal) "0.400000,0.400000,0.400000" true "AutoRelease")
        (Utilities|FlowControl|Delay 0.5)
        (goto _label Reset)))))

(event Custom|PlaySwordHitSound
  ;[0.05098 0.05098 0.05098] PlaySwordHitSounds
  (Audio|PlaySoundatLocation "/Game/Audio/SwordHits/MS_SwordHit.MS_SwordHit" (Transformation|GetActorLocation (Components|GetOwner)) "0, 0, 0" 1.0 1.0 0.0 "/Game/Audio/SA_CharacterOverall.SA_CharacterOverall" 0 0 0))

(event Custom|StopCombo
  ;[0.05098 0.05098 0.05098] ComboSystem
  ;;[0.05098 0.05098 0.05098] Stop Combo Attack
  (Variables|Default|SetisAttacking? false)
  (Variables|Default|SetAttackIndex 0))

(event Custom|Attack03
  ;[0.05098 0.05098 0.05098] ComboSystem
  ;;[0.05098 0.05098 0.05098] Attack03
  (Utilities|FlowControl|DoOnce false :!label _label
    (:Completed
      (Utilities|FlowControl|Delay 0.1)
      (Animation|Montage|PlayMontage (Variables|Character|GetMesh) "/Game/Characters/RPG_Character/Animations/SwordAttacks/Attack3_Montage.Attack3_Montage"
        (:then
          (Variables|Default|SetAttackIndex 4)
          (goto _label Reset))))))

(event Custom|Attack00
  ;[0.05098 0.05098 0.05098] ComboSystem
  ;;[0.05098 0.05098 0.05098] Attack00
  (Utilities|FlowControl|DoOnce false :!label _label
    (:Completed
      (Utilities|FlowControl|Delay 0.1)
      (Animation|Montage|PlayMontage (Variables|Character|GetMesh) "/Game/Characters/RPG_Character/Animations/SwordAttacks/Attack1_Montage.Attack1_Montage"
        (:then
          (Variables|Default|SetAttackIndex 1)
          (goto _label Reset))))))

(event Custom|Ragdoll
  (params (RagdollWaitDuration :type Float%20%28single-precision%29) (DeathSoundWaitDuration :type Float%20%28single-precision%29))
  (bind _capsulecomponent (Variables|Collision|GetCapsuleComponent))
  (bind _mesh (Variables|Character|GetMesh))
  ;[0.05098 0.05098 0.05098] Ragdoll
  (Utilities|FlowControl|Sequence
    (:then_0
      (Utilities|FlowControl|Delay RagdollWaitDuration)
      (Physics|SetSimulatePhysics _mesh true)
      (Collision|SetCollisionObjectType _mesh "ECC_Pawn")
      (Collision|SetCollisionResponsetoChannel _mesh "ECC_Pawn" "ECR_Ignore")
      (Collision|SetCollisionEnabled (Variables|Default|GetAssassinationRadius) "NoCollision")
      (Collision|SetCollisionObjectType _capsulecomponent "ECC_Pawn")
      (Collision|SetCollisionResponsetoChannel _capsulecomponent "ECC_Camera" "ECR_Ignore")
      (Collision|SetCollisionResponsetoChannel _capsulecomponent "ECC_Pawn" "ECR_Ignore"))
    (:then_1
      (Utilities|FlowControl|Delay DeathSoundWaitDuration)
      (Audio|PlaySoundatLocation "/Game/Audio/HitGrunts/Death02.Death02" (Transformation|GetActorLocation) "0, 0, 0" 1.0 1.0 0.0 "/Game/Audio/SA_CharacterOverall.SA_CharacterOverall" 0 0 0)
      (Development|SetHiddeninGame (Variables|Default|GetHealthBarWidget) true true))))

(event Custom|Attack01
  ;[0.05098 0.05098 0.05098] ComboSystem
  ;;[0.05098 0.05098 0.05098] Attack01
  (Utilities|FlowControl|DoOnce false :!label _label
    (:Completed
      (Utilities|FlowControl|Delay 0.1)
      (Animation|Montage|PlayMontage (Variables|Character|GetMesh) "/Game/Characters/RPG_Character/Animations/SwordAttacks/Attack2_Montage.Attack2_Montage"
        (:then
          (Variables|Default|SetAttackIndex 2)
          (goto _label Reset))))))

(event Custom|AI_SwordAttackCombo_Main
  ;[0.05098 0.05098 0.05098] ComboSystem
  ;;[0.05098 0.05098 0.05098] AttackInput
  (if (Variables|Default|GetcanAttack?)
    (CallFunction|SwordAttack)))

(event Custom|Attack02
  ;[0.05098 0.05098 0.05098] ComboSystem
  ;;[0.05098 0.05098 0.05098] Attack02 (Not Using)
  (Utilities|FlowControl|DoOnce false :!label _label
    (:Completed
      (Utilities|FlowControl|Delay 0.1)
      (Animation|Montage|PlayMontage (Variables|Character|GetMesh) "/Game/Characters/RPG_Character/Animations/SwordAttacks/Kick_Montage.Kick_Montage"
        (:then
          (Variables|Default|SetAttackIndex 3)
          (goto _label Reset))))))

(event Custom|ToggleInvestigationIcon
  (params (IsInvestigating? :type Boolean))
  (Rendering|SetVisibility (Variables|Default|GetInvestigateWidget) IsInvestigating? false))

(event EventBeginPlay
  ;[0.05098 0.05098 0.05098] SetHealthBarWidgetVariable
  (bind _aswb_npc_health_bar (Utilities|Casting|CastToWB_NPC_HealthBar (UserInterface|GetWidget (Variables|Default|GetHealthBarWidget))))
  (Variables|Default|SetHealthBar _aswb_npc_health_bar))

(event EventTick
  (params (DeltaSeconds :type Float%20%28single-precision%29))
  (bind _returnvalue (Game|GetPlayerCameraManager 0))
  (bind _healthbarwidget (Variables|Default|GetHealthBarWidget))
  (bind _returnvalue_2 (Transformation|GetWorldLocation _healthbarwidget))
  (bind _transformcomponent (Variables|/Script/Engine.PlayerCameraManager|GetTransformComponent _returnvalue))
  (bind _returnvalue_3 (Transformation|GetWorldLocation _transformcomponent))
  (bind _returnvalue_4 (Math|Rotator|FindLookatRotation _returnvalue_2 _returnvalue_3))
  ;[0.05098 0.05098 0.05098] WidgetsLookAtPlayer
  (Transformation|SetWorldRotation (Variables|Default|GetHealthBarWidget) _returnvalue_4 false false)
  (Transformation|SetWorldRotation (Variables|Default|GetInvestigateWidget) _returnvalue_4 false false))

(event Game|Damage|EventAnyDamage
  (params (Damage :type Float%20%28single-precision%29) (DamageType :type Damage%20Type%20Object%20Reference) (InstigatedBy :type Controller%20Object%20Reference) (DamageCauser :type Actor%20Object%20Reference))
  (bind _hitanims (Variables|Default|GetHitAnims))
  (Animation|PlayAnimMontage (Utilities|Array|Get(acopy) _hitanims (Math|Random|RandomIntegerinRange 0 (- (Utilities|Array|Length _hitanims) 1))) 1.0 "None")
  (bind _asbp_third_person_character (Utilities|Casting|CastToBP_ThirdPersonCharacter (Game|GetPlayerCharacter 0)))
  (Character|LaunchCharacter (* (Math|Vector|GetForwardVector (Transformation|GetActorRotation _asbp_third_person_character)) 7e+02) false false)
  (Audio|PlaySoundatLocation "/Game/Audio/HitGrunts/Death01.Death01" (Transformation|GetActorLocation) "0, 0, 0" 1.0 1.0 0.0 "/Game/Audio/SA_CharacterOverall.SA_CharacterOverall" 0 0 0)
  (bind _isdead (Default|DecreaseHealth (Variables|Default|GetBPC_PlayerStats) Damage false true))
  (if _isdead
    (CallFunction|Ragdoll 0.0 0.0)))

(fn ConstructionScript)

(fn Attack
  (CallFunction|AISwordAttackComboMain)
  (return 0.4))

(fn StealthBackAssassination
  (Rendering|SetVisibility (Variables|Default|GetAssassinatePromptWidget) false false)
  (Animation|PlayAnimMontage "/Game/Characters/RPG_Character/Animations/Assassinations/Paired_Knife_Stealth_KidneyAndNeck_Vic_Montage.Paired_Knife_Stealth_KidneyAndNeck_Vic_Montage" 1.0 "None")
  (CallFunction|Ragdoll 2.5 2.0)
  (return (Transformation|GetWorldLocation (Variables|Default|GetAssassinREF)) (Transformation|GetActorRotation)))